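; Player character Blueprint for a Gundam Exia mech, layering input and boost VFX over guard and combo attack functions.
; Enhanced Input events call StartGuard, StopGuard and ExecuteAttack; older Blueprint versions of that logic remain unconnected, with a comment noting a C++ rewrite of the combo.
; Tick toggles thruster and afterimage Niagara effects during boost, guard, falling or the attack montage.
; Tick also stops boosting while guarding and clears guard while attacking.
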(event `self.ReceiveBeginPlay`
  ; 시작 시 호출
  (`parent.ReceiveBeginPlay`)
  (`/Engine/EditorBlueprintResources/StandardMacros.IsValid` self
    (:`Is Valid`
      (`KismetSystemLibrary.Delay` 0.2)
      (`|ExecutionSequence`
        (:`then_0`
          (`ActorComponent.Deactivate` (`self.NS_Exia_Thruster_Boost`)))
        (:`then_1`
          (`SceneComponent.SetHiddenInGame` (`self.Guarding`) true false))))))

(event `self.ReceiveTick`
  (params (DeltaSeconds :type "Float (single-precision)"))
  (bind _ns_exia_afterimage (`self.NS_Exia_AfterImage`))
  ; 이벤트 틱 ( 상시 )
  (`|ExecutionSequence`
    (:`then_0`
      ;; 부스터 중, 점프 중, 가드 중일때 VFX활성화
      (if (`self.CanBoost`)
        (`self.BoostingVFXOn` _ns_exia_afterimage)
        (elif (`ActorComponent.IsActive` _ns_exia_afterimage)
          (`self.BoostingVFXOff`))))
    (:`then_1`
      ;; 가드 중일땐 부스트 불가 ( 이펙트만 활성화 )
      (if (`self.bBlock`)
        (`self.StopBoost`)))
    (:`then_2`
      ;; 공격중일땐 가드 상태 해제
      (if (`self.Attacking`)
        (set `self.bBlock` false)))))

(event `EnhancedInput|/Game/SDGundamBA_Assets/Input/IA_Guard`
  (params (ActionValue :type Boolean) (ElapsedSeconds :type "Float (double-precision)") (TriggeredSeconds :type "Float (double-precision)") (InputAction :type "InputAction Object Reference" :default "/Game/SDGundamBA_Assets/Input/IA_Guard.IA_Guard"))
  ; 가드
  (:`Started`
    (`self.StartGuard`))
  (:`Completed`
    (`self.StopGuard`)))

(event `EnhancedInput|/Game/SDGundamBA_Assets/Input/IA_AttackCombo`
  (params (ActionValue :type Boolean) (ElapsedSeconds :type "Float (double-precision)") (TriggeredSeconds :type "Float (double-precision)") (InputAction :type "InputAction Object Reference" :default "/Game/SDGundamBA_Assets/Input/IA_AttackCombo.IA_AttackCombo"))
  ; 콤보어택 CPP리뉴얼
  (:`Started`
    (`GundamCombatInterface.ExecuteAttack` self)))

(event `ResetGuardCooldown`
  ; 가드 상태일때
  (set `self.IsCanGuard` true)
  (`KismetSystemLibrary.K2_ClearAndInvalidateTimerHandle` (`self.GuardTimerHandle`)))

(fn `BoostingVFXOff`
  (`ActorComponent.Deactivate` (`self.NS_Exia_AfterImage`))
  (`ActorComponent.Deactivate` (`self.NS_Exia_Thruster_Boost`)))

(fn `BoostingVFXOn`
  (params (self2 :type "ActorComponent Object Reference"))
  (if (not (`ActorComponent.IsActive` (`self.NS_Exia_AfterImage`)))
    (`ActorComponent.Activate` (`self.NS_Exia_Thruster_Boost`) false)
    (`ActorComponent.Activate` self2 false)))

(fn `CanBoost`
  (returns (CanBoosting :type Boolean))
  (return (or (`self.IsBoosting`) (`self.bBlock`) (`NavMovementComponent.IsFalling` (`self.CharacterMovement`)) (`AnimInstance.Montage_IsPlaying` (`SkeletalMeshComponent.GetAnimInstance` (`self.Mesh`)) (`self.AttackMontage`)))))

(fn `GNSword_Active`
  (`/Engine/EditorBlueprintResources/StandardMacros.IsValid` (`self.GN_Sword`)
    (:`Is Valid`
      (`ActorComponent.Deactivate` (`self.GN_Sword`)))))

(fn `UserConstructionScript`)