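; AI-controlled Gundam Exia character that layers thruster and afterimage VFX and floating damage numbers onto inherited combat behavior.
; ThrusterFX starts off, then Tick re-activates it whenever the afterimage is inactive, since its branch is fixed true and the shutoff path never runs.
; CanBoost and its duplicate NewFunction check boost, block, falling and attack montage but are not called here.
; Damage events forward to the parent, while ShowDamageText spawns BP_DamageFloater.
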(event `self.ReceiveBeginPlay`
  ; 시작 시 호출
  (`/Engine/EditorBlueprintResources/StandardMacros.IsValid` self
    (:`Is Valid`
      (`ActorComponent.Deactivate` (`self.ThrusterFX`)))))

(event `GundamCombatInterface.ApplyGundamDamage`
  (params (DamageAmount :type "Float (single-precision)") (Attacker :type "Actor Object Reference") (HitBoneName :type Name) (HitLocation :type "Vector Structure"))
  (`parent.ApplyGundamDamage` DamageAmount Attacker HitBoneName HitLocation))

(event `self.ReceiveTick`
  (params (DeltaSeconds :type "Float (single-precision)"))
  (bind _ns_exia_afterimage (`self.NS_Exia_AfterImage`))
  ; 이벤트 틱 ( 상시 )
  (`|ExecutionSequence`
    (:`then_0`
      ;; 부스터 중, 점프 중, 가드 중일때 VFX활성화
      (if true
        (`self.BoostingVFXOn` _ns_exia_afterimage)
        (elif (`ActorComponent.IsActive` _ns_exia_afterimage)
          (`self.BoostingVFXOff`))))))

(event `self.ShowDamageText`
  (params (Damage :type "Float (single-precision)") (Location :type "Vector Structure"))
  (`|SpawnActorFromClass` "/Game/SDGundamBA_Assets/Character/BP_PlayerCharacterActor/BP_DamageFloater.BP_DamageFloater_C" (`KismetMathLibrary.Conv_VectorToTransform` Location) "Undefined" "MultiplyWithRoot" null (`KismetMathLibrary.Conv_IntToDouble` (`KismetMathLibrary.FTrunc` Damage)) null))

(fn `BoostingVFXOff`
  (`ActorComponent.Deactivate` (`self.NS_Exia_AfterImage`))
  (`ActorComponent.Deactivate` (`self.ThrusterFX`)))

(fn `BoostingVFXOn`
  (params (Self3 :type "ActorComponent Object Reference"))
  (if (not (`ActorComponent.IsActive` (`self.NS_Exia_AfterImage`)))
    (`ActorComponent.Activate` (`self.ThrusterFX`) false)))

(fn `CanBoost`
  (returns (CanBoosting :type Boolean))
  (return (or (`self.IsBoosting`) (`self.bBlock`) (`NavMovementComponent.IsFalling` (`self.CharacterMovement`)) (`AnimInstance.Montage_IsPlaying` (`SkeletalMeshComponent.GetAnimInstance` (`self.Mesh`)) (`self.AttackMontage`)))))

(fn `NewFunction`
  (returns (ReturnValue :type Boolean))
  (return (or (`self.IsBoosting`) (`self.bBlock`) (`NavMovementComponent.IsFalling` (`self.CharacterMovement`)) (`AnimInstance.Montage_IsPlaying` (`SkeletalMeshComponent.GetAnimInstance` (`self.Mesh`)) (`self.AttackMontage`)))))

(fn `UserConstructionScript`)