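; Afterimage VFX actor that leaves a frozen ghost of a character's skeletal mesh.
; The rimage event copies the source mesh's pose onto the Afterimage component and applies a dynamic instance of AfterImageMat to its first material slot.
; Opacity is set once to StartOpacity through a zero-alpha Lerp, so it never fades before the actor destroys itself after a one-second delay.
; The Tint parameter setter is unconnected.
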(event `rimage`
  (params (SouceMesh :type "SkeletalMeshComponent Object Reference"))
  (bind _afterimage (`self.afterimage`))
  (`/Engine/EditorBlueprintResources/StandardMacros.IsValid` null
    (:`Is Valid`
      (`PoseableMeshComponent.CopyPoseFromSkeletalComponent` _afterimage SouceMesh)
      (bind _returnvalue (`PrimitiveComponent.CreateDynamicMaterialInstance` _afterimage 0 (`self.After Image Mat`) "None"))
      (bind _output_get (set `self.MID` _returnvalue))
      (`MaterialInstanceDynamic.SetScalarParameterValue` _output_get "Opacity" (`KismetMathLibrary.Lerp` (`self.Start Opacity`) (`self.End Opacity`)))
      (`KismetSystemLibrary.Delay` 1.0)
      (`self.K2_DestroyActor`))))

(fn `UserConstructionScript`)